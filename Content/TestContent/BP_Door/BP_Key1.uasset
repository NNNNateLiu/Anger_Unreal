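; BP_Key1 is a key pickup that the player collects with E to flag the Door1-tagged BP_Door1 as having its key.
; Box overlap with BP_ThirdPersonCharacter opens a gate and enables input, and leaving closes and disables both.
; Pressing E inside sets Key1 on the first tagged door, prints a debug string and destroys the key, provided the game instance casts to BP_MyInstance.
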(event OnComponentBeginOverlap(Box)
  (params (OverlappedComponent :type Primitive%20Component%20Object%20Reference) (OtherActor :type Actor%20Object%20Reference) (OtherComp :type Primitive%20Component%20Object%20Reference) (OtherBodyIndex :type Integer) (bFromSweep :type Boolean) (SweepResult :type Hit%20Result%20Structure%20%28by%20ref%29))
  ;[1 1 1] overlap
  (bind _asbp_third_person_character (Utilities|Casting|CastToBP_ThirdPersonCharacter OtherActor))
  (Utilities|IsValid _asbp_third_person_character
    (:Is%20Valid
      (Utilities|FlowControl|Sequence
        (:then_0
          (Utilities|FlowControl|Gate true) ; enters at Open
        )
        (:then_1
          ;[1 1 1] text visible
          (Input|EnableInput (Game|GetPlayerController 0)))))))

(event OnComponentEndOverlap(Box)
  (params (OverlappedComponent :type Primitive%20Component%20Object%20Reference) (OtherActor :type Actor%20Object%20Reference) (OtherComp :type Primitive%20Component%20Object%20Reference) (OtherBodyIndex :type Integer))
  ;[1 1 1] overlap
  (bind _asbp_third_person_character (Utilities|Casting|CastToBP_ThirdPersonCharacter OtherActor))
  (Utilities|IsValid _asbp_third_person_character
    (:Is%20Valid
      (Utilities|FlowControl|Sequence
        (:then_0
          (Utilities|FlowControl|Gate true) ; enters at Close
        )
        (:then_1
          ;[1 1 1] text visible
          (Input|DisableInput (Game|GetPlayerController 0)) ; disable input
        )))))

(event Input|KeyboardEvents|E
  (params (Key :type Key%20Structure :default "None"))
  (:Pressed
    (Utilities|FlowControl|Gate true
      (:Exit
        (Utilities|Casting|CastToBP_MyInstance (Game|GetGameInstance))
        (bind _outactors (Actor|GetAllActorsOfClasswithTag "/Game/TestContent/BP_Door/BP_Door1.BP_Door1_C" "Door1"))
        (Variables|/Game/TestContent/BP_Door/BP_Door1.BP_Door1_C|SetKey1 (Utilities|Array|Get(acopy) _outactors) true)
        (Development|PrintString "key")
        (Actor|DestroyActor)))))

(fn ConstructionScript)