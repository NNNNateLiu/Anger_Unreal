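; BP_Door1 is a test door that the player toggles open and closed with the E key while standing inside its Box trigger.
; Box overlap enables input and opens a gate, and leaving the box closes the gate.
; When Key1 is true, each press flip-flops a timeline between play and reverse to drive the door's yaw rotation.
; Without the key it prints "No Key".
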(event OnComponentBeginOverlap(Box)
  (params (OverlappedComponent :type Primitive%20Component%20Object%20Reference) (OtherActor :type Actor%20Object%20Reference) (OtherComp :type Primitive%20Component%20Object%20Reference) (OtherBodyIndex :type Integer) (bFromSweep :type Boolean) (SweepResult :type Hit%20Result%20Structure%20%28by%20ref%29))
  (Input|EnableInput (Game|GetPlayerController 0))
  (Utilities|FlowControl|Gate true) ; enters at Open
)

(event OnComponentEndOverlap(Box)
  (params (OverlappedComponent :type Primitive%20Component%20Object%20Reference) (OtherActor :type Actor%20Object%20Reference) (OtherComp :type Primitive%20Component%20Object%20Reference) (OtherBodyIndex :type Integer))
  (Utilities|FlowControl|Gate true) ; enters at Close
)

(event Input|KeyboardEvents|E
  (params (Key :type Key%20Structure))
  (:Pressed
    (if (Variables|Default|GetKey1)
      (Utilities|FlowControl|Gate true
        (:Exit
          (Utilities|FlowControl|FlipFlop ; like receptacle
            (:A
              (bind _新建轨道_0 (Timeline|时间轴_0 Play)
                (:Update
                  (Transformation|SetRelativeRotation (Variables|Default|GetDoor) (Math|Rotator|MakeRotator 0.0 0.0 _新建轨道_0) false false))))
            (:B
              (Timeline|时间轴_0 Reverse)))))
      (else
        (Development|PrintString "No Key")))))

(fn ConstructionScript)