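; Test map portal Blueprint that moves the player to Map_Egypt2 when its Box is overlapped.
; On any overlap it shows a fade widget, waits briefly, then opens the level.
; It then calls RestartPlayerAtPlayerStart for player start "1", after the OpenLevel call rather than in the new level.
; An unconnected chain would save the character's health and mana to BP_SaveGame, but never runs.
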(event OnComponentBeginOverlap(Box)
  (params (OverlappedComponent :type Primitive%20Component%20Object%20Reference) (OtherActor :type Actor%20Object%20Reference) (OtherComp :type Primitive%20Component%20Object%20Reference) (OtherBodyIndex :type Integer) (bFromSweep :type Boolean) (SweepResult :type Hit%20Result%20Structure%20%28by%20ref%29))
  (bind _returnvalue (Game|GetPlayerController 0))
  (bind _returnvalue_2 (Game|GetGameMode))
  (bind _returnvalue_3 (UserInterface|CreateWidget "/Game/TestContent/Test_MapPortal/WB_fade.WB_fade_C")) ; create widget
  (UserInterface|Viewport|AddtoViewport _returnvalue_3 0)
  (Default|FadeEvent _returnvalue_3)
  (Utilities|FlowControl|Delay 0.5)
  (Game|OpenLevel(byName) "Map_Egypt2")
  (Class|GameModeBase|RestartPlayeratPlayerStart _returnvalue_2 _returnvalue (Class|GameModeBase|FindPlayerStart _returnvalue_2 _returnvalue "1")))

(fn ConstructionScript)