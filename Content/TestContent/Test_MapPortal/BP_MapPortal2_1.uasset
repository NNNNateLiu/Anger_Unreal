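; BP_MapPortal2_1 is a test map portal that sends the player to Map_Egypt1 when its Box is overlapped.
; The overlap, not filtered by actor, saves player 0's health, health background and mana to a new BP_SaveGame in slot "save1".
; It then plays the WB_fade widget, waits briefly and opens the level.
; After the OpenLevel call it requests a restart at PlayerStart "1" from the current GameMode.
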(event OnComponentBeginOverlap(Box)
  (params (OverlappedComponent :type Primitive%20Component%20Object%20Reference) (OtherActor :type Actor%20Object%20Reference) (OtherComp :type Primitive%20Component%20Object%20Reference) (OtherBodyIndex :type Integer) (bFromSweep :type Boolean) (SweepResult :type Hit%20Result%20Structure%20%28by%20ref%29))
  (bind _returnvalue (Game|GetPlayerController 0))
  (bind _returnvalue_2 (Game|GetGameMode))
  (bind _returnvalue_3 (SaveGame|CreateSaveGameObject "/Game/ThirdPerson/Blueprints/BP_SaveGame.BP_SaveGame_C"))
  (bind _asbp_third_person_character (Utilities|Casting|CastToBP_ThirdPersonCharacter (Game|GetPlayerCharacter 0)))
  (Variables|/Game/ThirdPerson/Blueprints/BP_SaveGame.BP_SaveGame_C|SetHP _returnvalue_3 (Variables|/Game/ThirdPerson/Blueprints/BP_ThirdPersonCharacter.BP_ThirdPersonCharacter_C|GetHealth _asbp_third_person_character))
  (Variables|/Game/ThirdPerson/Blueprints/BP_SaveGame.BP_SaveGame_C|SetHP_Background _returnvalue_3 (Variables|/Game/ThirdPerson/Blueprints/BP_ThirdPersonCharacter.BP_ThirdPersonCharacter_C|GetHealth_Background _asbp_third_person_character))
  (Variables|/Game/ThirdPerson/Blueprints/BP_SaveGame.BP_SaveGame_C|SetMP _returnvalue_3 (Variables|/Game/ThirdPerson/Blueprints/BP_ThirdPersonCharacter.BP_ThirdPersonCharacter_C|GetMana _asbp_third_person_character))
  (SaveGame|SaveGametoSlot _returnvalue_3 "save1") ; 开始存盘
  (bind _returnvalue_4 (UserInterface|CreateWidget "/Game/TestContent/Test_MapPortal/WB_fade.WB_fade_C")) ; create widget
  (UserInterface|Viewport|AddtoViewport _returnvalue_4 0)
  (Default|FadeEvent _returnvalue_4)
  (Utilities|FlowControl|Delay 0.5)
  (Game|OpenLevel(byName) "Map_Egypt1")
  (Class|GameModeBase|RestartPlayeratPlayerStart _returnvalue_2 _returnvalue (Class|GameModeBase|FindPlayerStart _returnvalue_2 _returnvalue "1")))

(fn ConstructionScript)